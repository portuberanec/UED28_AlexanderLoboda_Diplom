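; Health pickup that restores health to an actor and then removes itself from the world.
; ActivatePickupEffect looks for a BPAC_Health component on the given actor, adds AddedHealth through it and destroys the pickup, doing nothing if the component is missing.
; Overlap handling is deferred to the parent class.
; Tick rotates the pickup by a fixed step each frame, so spin speed depends on frame rate.
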(event EventBeginPlay
  (|CallParentFunction))

(event Collision|EventActorBeginOverlap
  (params (OtherActor :type Actor%20Object%20Reference))
  (|CallParentFunction OtherActor))

(event EventTick
  (params (DeltaSeconds :type Float%20%28single-precision%29))
  (|CallParentFunction DeltaSeconds)
  (Class|Actor|AddActorWorldRotation "0.000000,1.000000,0.000000"))

(fn ConstructionScript
  (|CallParentFunction))

(fn ActivatePickupEffect
  (params (InActor :type Actor%20Object%20Reference))
  (bind _returnvalue (Actor|GetComponentbyClass InActor "/Game/MyBlueprints/Components/BPAC_Health.BPAC_Health_C"))
  (Utilities|IsValid _returnvalue
    (:Is%20Valid
      (LocalVariables|SetL_HealthComp _returnvalue)
      (Default|AddHealth (LocalVariables|GetL_HealthComp) (Variables|Config|GetAddedHealth))
      (Actor|DestroyActor))))