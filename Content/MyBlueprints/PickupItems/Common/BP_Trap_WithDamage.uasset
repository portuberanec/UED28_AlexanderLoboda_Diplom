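; BP_Trap_WithDamage is a pickup-style trap that damages the actor it affects.
; It overrides ActivatePickupEffect, running the parent effect before looking up the actor's BPAC_Health component and calling DecHealth with DecHP.
; The health component is used without a validity check.
; The event graph holds only disabled stubs and the construction script just calls the parent, so triggering is not defined here.
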(event EventBeginPlay
  (|CallParentFunction) ; This node is disabled and will not be called.\nDrag off pins to build functionality.
)

(event Collision|EventActorBeginOverlap
  (params (OtherActor :type Actor%20Object%20Reference))
  (|CallParentFunction OtherActor) ; This node is disabled and will not be called.\nDrag off pins to build functionality.
)

(event EventTick
  (params (DeltaSeconds :type Float%20%28single-precision%29))
  (|CallParentFunction DeltaSeconds) ; This node is disabled and will not be called.\nDrag off pins to build functionality.
)

(fn ConstructionScript
  (|CallParentFunction))

(fn ActivatePickupEffect
  (params (InActor :type Actor%20Object%20Reference))
  (bind _output_get (LocalVariables|SetL_CurrentActor InActor))
  (|CallParentFunction _output_get)
  (Default|DecHealth (Actor|GetComponentbyClass (LocalVariables|GetL_CurrentActor) "/Game/MyBlueprints/Components/BPAC_Health.BPAC_Health_C") (Variables|Config|GetDecHP)))