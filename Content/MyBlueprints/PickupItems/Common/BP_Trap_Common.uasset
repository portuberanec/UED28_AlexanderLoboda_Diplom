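; Common trap pickup that affects actors overlapping it, either on entry or periodically.
; Overlap events maintain a list of actors inside, and TrapEffect calls ActivatePickup on each one.
; With Periodical set, each entry sets a looping timer instead of calling TrapEffect directly, and the timer is cleared when the last actor leaves.
; Otherwise, every new overlap immediately reapplies the effect to all listed actors.
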(event EventBeginPlay
  (|CallParentFunction) ; This node is disabled and will not be called.\nDrag off pins to build functionality.
)

(event Collision|EventActorBeginOverlap
  (params (OtherActor :type Actor%20Object%20Reference))
  (Utilities|Array|AddUnique (Variables|Default|GetOverlappedActors) OtherActor)
  (if (> (Utilities|Array|Length (Variables|Default|GetOverlappedActors)) 0)
    (if (Variables|Config|GetPeriodical)
      (bind _returnvalue (Utilities|Time|SetTimerbyEvent (EventDispatchers|CreateEvent :!event TrapEffect) (Variables|Config|GetPeriodicalTime) (Variables|Config|GetPeriodical)))
      (Variables|Default|SetTimerForTrap _returnvalue)
      (else
        (CallFunction|TrapEffect)))))

(event EventTick
  (params (DeltaSeconds :type Float%20%28single-precision%29))
  (|CallParentFunction DeltaSeconds) ; This node is disabled and will not be called.\nDrag off pins to build functionality.
)

(event Collision|EventActorEndOverlap
  (params (OtherActor :type Actor%20Object%20Reference))
  (Utilities|Array|RemoveItem (Variables|Default|GetOverlappedActors) OtherActor)
  (if (== (Utilities|Array|Length (Variables|Default|GetOverlappedActors)) 0)
    (if (Utilities|Time|IsValidTimerHandle (Variables|Default|GetTimerForTrap))
      (Utilities|Time|ClearandInvalidateTimerbyHandle (Variables|Default|GetTimerForTrap)))))

(fn ConstructionScript
  (|CallParentFunction))

(fn TrapEffect
  (for _array_element (Variables|Default|GetOverlappedActors)
    (CallFunction|ActivatePickup _array_element)))