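; BP_DoorWithLock is a door that requires keys to open.
; Overlapping its collision box while Locked asks the BPACLock component to unlock with the overlapping actor, opening the door on success.
; On failure it prints the display name of each required key class as debug output.
; Ending the overlap closes the door.
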(event OnComponentBeginOverlap(BoxCollision)
  (params (OverlappedComponent :type Primitive%20Component%20Object%20Reference) (OtherActor :type Actor%20Object%20Reference) (OtherComp :type Primitive%20Component%20Object%20Reference) (OtherBodyIndex :type Integer) (bFromSweep :type Boolean) (SweepResult :type Hit%20Result%20Structure%20%28by%20ref%29))
  (switch Utilities|FlowControl|Switch|SwitchonENUM_DoorStates (Variables|Default|GetDoorStates)
    (:NewEnumerator2
      (bind _unlocked (Default|Unlock (Variables|Default|GetBPAC_Lock) OtherActor))
      (if _unlocked
        (CallFunction|OpenDoor)
        (else
          ;[0.1719 0.1719 0.1719] Debug
          (if (Utilities|Enum|Equal(Enum) (Variables|Default|GetDoorStates) "NewEnumerator2")
            (for _array_element (Variables|/Game/MyBlueprints/Door/Components/BPAC_Lock.BPAC_Lock_C|GetKeysRequired (Variables|Default|GetBPAC_Lock))
              (Development|PrintString (Utilities|String|Append "You need " (Utilities|GetClassDisplayName _array_element)) true false))))))))

(event OnComponentEndOverlap(BoxCollision)
  (params (OverlappedComponent :type Primitive%20Component%20Object%20Reference) (OtherActor :type Actor%20Object%20Reference) (OtherComp :type Primitive%20Component%20Object%20Reference) (OtherBodyIndex :type Integer))
  (CallFunction|CloseDoor))

(fn ConstructionScript
  (|CallParentFunction))