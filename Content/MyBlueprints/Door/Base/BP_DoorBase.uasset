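; Base door Blueprint that swings open when something overlaps its box collision and closes when the overlap ends.
; A timeline, played or reversed by OpenDoor and CloseDoor, scales MaxDoorOpenAngle onto the Rotator's yaw and updates a door state enum.
; The construction script applies the initial Opened pose and state.
; AnimDuration feeds the timeline's play rate directly, and Tick prints the state for debugging.
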(event OnComponentBeginOverlap(BoxCollision)
  (params (OverlappedComponent :type Primitive%20Component%20Object%20Reference) (OtherActor :type Actor%20Object%20Reference) (OtherComp :type Primitive%20Component%20Object%20Reference) (OtherBodyIndex :type Integer) (bFromSweep :type Boolean) (SweepResult :type Hit%20Result%20Structure%20%28by%20ref%29))
  (CallFunction|OpenDoor))

(event OnComponentEndOverlap(BoxCollision)
  (params (OverlappedComponent :type Primitive%20Component%20Object%20Reference) (OtherActor :type Actor%20Object%20Reference) (OtherComp :type Primitive%20Component%20Object%20Reference) (OtherBodyIndex :type Integer))
  (CallFunction|CloseDoor))

(event EventBeginPlay
  (Components|Timeline|SetPlayRate (Variables|Default|GetTimeline_DoorOpen) (Variables|Default|GetAnimDuration)))

(event EventTick
  (params (DeltaSeconds :type Float%20%28single-precision%29))
  (Development|PrintString (Utilities|String|EnumtoString (Variables|Default|GetDoorStates)) true false "(R=0.973687,G=0.000000,B=1.000000,A=1.000000)" 0.0))

(fn ConstructionScript
  (bind _timeline_dooropen (Variables|Default|GetTimeline_DoorOpen))
  (Transformation|SetRelativeRotation (Variables|Default|GetRotator) (Math|Rotator|MakeRotator 0.0 0.0 (select (Variables|Default|GetOpened) (Variables|Default|GetMaxDoorOpenAngle) 0.0)) false false)
  (if (Variables|Default|GetOpened)
    (Variables|Default|SetDoorStates "NewEnumerator0")
    (Components|Timeline|SetNewTime _timeline_dooropen (Components|Timeline|GetTimelineLength _timeline_dooropen))
    (else
      (Variables|Default|SetDoorStates "NewEnumerator1"))))

(fn OpenDoor
  (bind _doorstates (Variables|Default|GetDoorStates))
  (if (or (Utilities|Enum|Equal(Enum) _doorstates "NewEnumerator1") (Utilities|Enum|Equal(Enum) _doorstates "NewEnumerator3"))
    (Audio|Components|Audio|Play (Variables|Default|GetTimeline_DoorOpen))
    (else
      (CallFunction|CloseDoor))))

(fn CloseDoor
  (Utilities|String|Reverse (Variables|Default|GetTimeline_DoorOpen)))

(fn ProcessAnimation
  (params (A :type Float%20%28double-precision%29))
  (Variables|Default|SetDoorStates "NewEnumerator3")
  (Transformation|SetRelativeRotation (Variables|Default|GetRotator) (Math|Rotator|MakeRotator 0.0 0.0 (* A (Variables|Default|GetMaxDoorOpenAngle))) false false))