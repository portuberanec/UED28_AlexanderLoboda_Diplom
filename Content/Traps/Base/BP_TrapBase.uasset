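; Base trap Blueprint that triggers when something enters its collision sphere, with an empty ActivateTrap function, apparently meant for child traps to override.
; Each begin overlap calls ActivateTrap immediately, then sets an event timer using PeriodicalTime, looping if Periodical is set, and stores its handle.
; End overlap clears that stored timer once the trap has no overlapping actors left.
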(event OnComponentBeginOverlap(SphereCollision)
  (params (OverlappedComponent :type Primitive%20Component%20Object%20Reference) (OtherActor :type Actor%20Object%20Reference) (OtherComp :type Primitive%20Component%20Object%20Reference) (OtherBodyIndex :type Integer) (bFromSweep :type Boolean) (SweepResult :type Hit%20Result%20Structure%20%28by%20ref%29))
  (CallFunction|ActivateTrap)
  (bind _returnvalue (Utilities|Time|SetTimerbyEvent (EventDispatchers|CreateEvent :!event ActivateTrap) (Variables|Default|GetPeriodicalTime) (Variables|Default|GetPeriodical)))
  (Variables|Default|SetTimerForTrapEvents _returnvalue))

(event OnComponentEndOverlap(SphereCollision)
  (params (OverlappedComponent :type Primitive%20Component%20Object%20Reference) (OtherActor :type Actor%20Object%20Reference) (OtherComp :type Primitive%20Component%20Object%20Reference) (OtherBodyIndex :type Integer))
  (if (== (Utilities|Array|Length (Collision|GetOverlappingActors 0 :!class /Script/Engine.Actor)) 0)
    (if (Utilities|Time|IsValidTimerHandle (Variables|Default|GetTimerForTrapEvents))
      (Utilities|Time|ClearandInvalidateTimerbyHandle (Variables|Default|GetTimerForTrapEvents)))))

(fn ConstructionScript)

(fn ActivateTrap)