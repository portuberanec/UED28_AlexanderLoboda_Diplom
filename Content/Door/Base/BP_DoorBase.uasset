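; Base door Blueprint that swings open and closed by yawing a Rotator component up to MaxDoorOpenAngle.
; OpenDoor and CloseDoor mark the door InProcess and play or reverse the timeline, with play rate set from AnimDuration.
; Timeline handlers, with no wired exec input, map OpenMult to rotation and set the final Opened or Closed state.
; Construction script pre-poses doors starting Opened; Tick prints each door's state for debugging.
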(event EventBeginPlay
  (Components|Timeline|SetPlayRate (Variables|Default|GetTimeline_Door) (Variables|Default|GetAnimDuration)))

(event EventTick
  (params (DeltaSeconds :type Float%20%28single-precision%29))
  (Development|PrintString (Utilities|String|Append (Utilities|GetDisplayName self) " | " (Utilities|String|EnumtoString (Variables|Default|GetDoorState))) true false "(R=0.973687,G=0.000000,B=1.000000,A=1.000000)" 0.0))

(fn ConstructionScript
  (bind _timeline_door (Variables|Default|GetTimeline_Door))
  (switch Utilities|FlowControl|Switch|SwitchonENUM_DoorState (Variables|Default|GetDoorState)
    (:NewEnumerator0
      (Components|Timeline|SetNewTime _timeline_door (Components|Timeline|GetTimelineLength _timeline_door))
      (Variables|Default|SetDoorState "NewEnumerator0")
      (CallFunction|ProcessAnimation 1.0))))

(fn OpenDoor
  (Variables|Default|SetDoorState "NewEnumerator3")
  (Audio|Components|Audio|Play (Variables|Default|GetTimeline_Door)))

(fn CloseDoor
  (switch Utilities|FlowControl|Switch|SwitchonENUM_DoorState (Variables|Default|GetDoorState)
    (:NewEnumerator0
      _)
    (:NewEnumerator3
      _))
  (Variables|Default|SetDoorState "NewEnumerator3")
  (Utilities|String|Reverse (Variables|Default|GetTimeline_Door)))

(fn ProcessAnimation
  (params (OpenMult :type Float%20%28double-precision%29))
  (Transformation|SetRelativeRotation (Variables|Default|GetRotator) (Math|Rotator|MakeRotator 0.0 0.0 (* OpenMult (Variables|Default|GetMaxDoorOpenAngle))) false false))