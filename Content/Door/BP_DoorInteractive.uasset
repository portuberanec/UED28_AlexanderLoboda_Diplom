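; Interactive door Blueprint that opens, closes or attempts an unlock when it receives an interact message.
; Its box collision adds the door to, and removes it from, the interaction queue of any overlapping actor with a BPAC_Interaction component.
; Interaction switches on door state: closed opens, opened or in-process closes, and locked asks BPACLock to unlock for the interactor, opening on success or calling DebugKeys on failure.
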(event OnComponentBeginOverlap(BoxCollision)
  (params (OverlappedComponent :type Primitive%20Component%20Object%20Reference) (OtherActor :type Actor%20Object%20Reference) (OtherComp :type Primitive%20Component%20Object%20Reference) (OtherBodyIndex :type Integer) (bFromSweep :type Boolean) (SweepResult :type Hit%20Result%20Structure%20%28by%20ref%29))
  (bind _returnvalue (Actor|GetComponentbyClass OtherActor "/Game/ComponentsCommon/BPAC_Interaction.BPAC_Interaction_C"))
  (Utilities|IsValid _returnvalue
    (:Is%20Valid
      (Default|AddtoQueue _returnvalue self))))

(event OnComponentEndOverlap(BoxCollision)
  (params (OverlappedComponent :type Primitive%20Component%20Object%20Reference) (OtherActor :type Actor%20Object%20Reference) (OtherComp :type Primitive%20Component%20Object%20Reference) (OtherBodyIndex :type Integer))
  (bind _returnvalue (Actor|GetComponentbyClass OtherActor "/Game/ComponentsCommon/BPAC_Interaction.BPAC_Interaction_C"))
  (Utilities|IsValid _returnvalue
    (:Is%20Valid
      (Default|RemovefromQueue _returnvalue self))))

(event EventInteractMessage
  (params (Interactor :type Actor%20Object%20Reference))
  (switch Utilities|FlowControl|Switch|SwitchonENUM_DoorState (Variables|Default|GetCurrentState)
    (:NewEnumerator0
      (CallFunction|CloseDoor :!label _label))
    (:NewEnumerator1
      (CallFunction|OpenDoor))
    (:NewEnumerator2
      (bind _unlocked (Default|Unlock (Variables|Default|GetBPAC_Lock) Interactor))
      (if _unlocked
        (CallFunction|OpenDoor)
        (else
          (CallFunction|DebugKeys Interactor))))
    (:NewEnumerator3
      (goto _label))))

(fn ConstructionScript
  (|CallParentFunction))