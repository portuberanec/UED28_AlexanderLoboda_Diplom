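; BP_Projectile_Rocket is a rocket projectile Blueprint that deals area damage and then destroys itself.
; Its ApplyDamage function ignores the owner as the hit actor, otherwise applying full radial damage at the static mesh's location while excluding the owner.
; A debug sphere shows the blast radius on each detonation.
; The event graph and construction script add no logic of their own.
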(event EventBeginPlay
  (|CallParentFunction) ; This node is disabled and will not be called.\nDrag off pins to build functionality.
)

(fn ConstructionScript
  (|CallParentFunction))

(fn ApplyDamage
  (params (OtherActor :type Actor%20Object%20Reference))
  (if (!= OtherActor (Components|GetOwner))
    (Rendering|Debug|DrawDebugSphere (Transformation|GetWorldLocation (Variables|Default|GetStaticMesh)) (Variables|Default|GetRadius) 12 "(R=0.000000,G=1.000000,B=0.915713,A=1.000000)" 3.0 1.0)
    (Game|Damage|ApplyRadialDamage (Variables|Default|GetDamage) (Transformation|GetWorldLocation (Variables|Default|GetStaticMesh)) (Variables|Default|GetRadius) "/Script/Engine.DamageType" (Utilities|Array|MakeArray (Components|GetOwner)) (Components|GetOwner) 0 true "ECC_Visibility")
    (Actor|DestroyActor)))