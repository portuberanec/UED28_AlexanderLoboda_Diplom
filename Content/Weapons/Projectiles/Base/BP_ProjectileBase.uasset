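; Base projectile actor that flies along a given direction and damages what it hits.
; BeginPlay sets the ProjectileMovement velocity from ProjectileDirection and the initial speed, while AcceptDamageAndVelocity lets a caller set the damage and redirect it at that speed.
; When the static mesh begins overlapping any actor other than its owner, it applies damage with the owner as damage causer, then destroys itself.
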(event OnComponentBeginOverlap(StaticMesh)
  (params (OverlappedComponent :type Primitive%20Component%20Object%20Reference) (OtherActor :type Actor%20Object%20Reference) (OtherComp :type Primitive%20Component%20Object%20Reference) (OtherBodyIndex :type Integer) (bFromSweep :type Boolean) (SweepResult :type Hit%20Result%20Structure%20%28by%20ref%29))
  (if (!= OtherActor (Components|GetOwner))
    (Game|Damage|ApplyDamage OtherActor (Variables|Default|GetDamage) 0 (Components|GetOwner))
    (Actor|DestroyActor)))

(event EventBeginPlay
  (Variables|/Script/Engine.MovementComponent|SetVelocity (Variables|Default|GetProjectileMovement) (* (Variables|Default|GetProjectileDirection) (Variables|/Script/Engine.ProjectileMovementComponent|GetInitialSpeed (Variables|Default|GetProjectileMovement)))))

(fn ConstructionScript)

(fn AcceptDamageandVelocity
  (params (Damage :type Float%20%28double-precision%29) (DirectionNormal :type Vector))
  (Variables|Default|SetDamage Damage)
  (Variables|/Script/Engine.MovementComponent|SetVelocity (Variables|Default|GetProjectileMovement) (* DirectionNormal (Variables|/Script/Engine.ProjectileMovementComponent|GetInitialSpeed (Variables|Default|GetProjectileMovement)))))