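; Pistol weapon Blueprint that implements Fire by always launching a projectile, leaving the hitscan flag, target and causer inputs unused.
; Fire spawns the supplied projectile class at the static mesh's MuzzleScene socket with zero rotation, owned by the actor the weapon is attached to.
; It then hands damage and direction to the projectile through AcceptDamageAndVelocity.
; The construction script only calls its parent.
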(fn ConstructionScript
  (|CallParentFunction))

(fn Fire
  (params (TargetActor :type Actor%20Object%20Reference) (Damage :type Float%20%28double-precision%29) (IsHitscan :type Boolean) (ProjectileType :type BP%20Projectile%20Base%20Class%20Reference) (ProjectileDirection :type Vector :default "0, 0, 0") (Causer :type Actor%20Object%20Reference))
  (bind _returnvalue (Game|SpawnActorfromClass ProjectileType (Math|Transform|MakeTransform (Transformation|GetSocketLocation (Variables|Default|GetStaticMesh) "MuzzleScene")) "AdjustIfPossibleButAlwaysSpawn" "MultiplyWithRoot" (Actor|GetAttachParentActor) 0))
  (Default|AcceptDamageandVelocity _returnvalue Damage ProjectileDirection))