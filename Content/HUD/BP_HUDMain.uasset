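; BP_HUDMain is the HUD actor that manages the WBP_MainHud widget for the player's weapon display.
; On BeginPlay it looks up the BPAC_WeaponManager component on the controlled pawn and binds to its weapon-chosen and weapon-lost events.
; ConstructHud lazily creates and caches the widget, then calls its ChooseWeapon.
; UnbindFromWeapon forwards to the widget's UnbindFromAll to release weapon bindings.
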(event EventBeginPlay
  (bind _playerowner (Variables|Default|GetPlayerOwner))
  (bind _returnvalue (Pawn|GetControlledPawn _playerowner))
  (bind _returnvalue_2 (Actor|GetComponentbyClass _returnvalue "/Game/Weapons/Components/BPAC_WeaponManager.BPAC_WeaponManager_C"))
  (Utilities|IsValid _returnvalue_2
    (:Is%20Valid
      (EventDispatchers|BindEventtoOnIsWeaponChosen _returnvalue_2 (EventDispatchers|CreateEvent :!event ConstructHud))
      (EventDispatchers|BindEventtoOnWeaponLost _returnvalue_2 (EventDispatchers|CreateEvent :!event UnbindfromWeapon)))))

(fn ConstructionScript)

(fn ConstructHud
  (Utilities|IsValid (Variables|Default|GetW_MainHud)
    (:Is%20Valid
      (Default|ChooseWeapon (Variables|Default|GetW_MainHud)))
    (:Is%20Not%20Valid
      (bind _returnvalue (UserInterface|CreateWidget "/Game/HUD/Widgets/WBP_MainHud.WBP_MainHud_C" (Game|Player|GetOwningPlayerController)))
      (bind _output_get (Variables|Default|SetW_MainHud _returnvalue))
      (Default|ChooseWeapon _output_get)
      (UserInterface|Viewport|AddtoViewport (Variables|Default|GetW_MainHud) 0))))

(fn UnbindfromWeapon
  (params (Main :type Boolean))
  (Utilities|IsValid (Variables|Default|GetW_MainHud)
    (:Is%20Valid
      (Default|UnbindfromAll (Variables|Default|GetW_MainHud) Main))))