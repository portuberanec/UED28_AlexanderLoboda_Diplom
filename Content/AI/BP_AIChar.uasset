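; AI character with a health component that reacts to damage and gets knocked back by radial damage, with debug HP text drawn above it.
; Any damage lowers BPACHealth and tells BP_AIController to react to the damage causer.
; Radial damage removes braking friction and applies a velocity impulse against the hit normal with clamped lift, then starts a one-second timer.
; BeginPlay caches the original braking values for restoring friction and binds an event to health reaching zero.
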(event EventTick
  (params (DeltaSeconds :type Float%20%28single-precision%29))
  (bind _returnvalue (Transformation|GetActorLocation))
  (Rendering|Debug|DrawDebugString (Math|Vector|MakeVector (.x _returnvalue) (.y _returnvalue) (+ (.z _returnvalue) 1.5e+02)) (Utilities|String|Append "HP: " (Utilities|String|ToString(Float) (Variables|/Game/ComponentsCommon/BPAC_EntityResource.BPAC_EntityResource_C|GetCurrentValue (Variables|Default|GetBPAC_Health))) " / " (Utilities|String|ToString(Float) (Variables|/Game/ComponentsCommon/BPAC_EntityResource.BPAC_EntityResource_C|GetMaxValue (Variables|Default|GetBPAC_Health)))) 0 "(R=1.000000,G=0.000000,B=0.023477,A=1.000000)"))

(event EventBeginPlay
  (bind _charactermovement (Variables|Character|GetCharacterMovement))
  (EventDispatchers|BindEventtoOnValueZero (Variables|Default|GetBPAC_Health) (EventDispatchers|CreateEvent (Variables|Default|GetBPAC_Action_Death) :!event Action))
  (Variables|Default|SetOrigFrictionFactor (Variables|/Script/Engine.CharacterMovementComponent|GetBrakingFrictionFactor _charactermovement))
  (Variables|Default|SetOrigDeceleraion (Variables|/Script/Engine.CharacterMovementComponent|GetBrakingDecelerationWalking _charactermovement)))

(fn ConstructionScript)

(fn ReceiveAnyDamage
  (params (Damage :type Float%20%28single-precision%29) (DamageType :type Damage%20Type%20Object%20Reference) (InstigatedBy :type Controller%20Object%20Reference) (DamageCauser :type Actor%20Object%20Reference))
  (Default|DecreaseValue (Variables|Default|GetBPAC_Health) Damage)
  (bind _asbp_aicontroller (Utilities|Casting|CastToBP_AIController (Pawn|GetController)))
  (Default|ReacttoAttack _asbp_aicontroller DamageCauser))

(fn ReceiveRadialDamage
  (params (DamageReceived :type Float%20%28single-precision%29) (DamageType :type Damage%20Type%20Object%20Reference) (Origin :type Vector :default "0, 0, 0") (HitInfo :type Hit%20Result%20Structure%20%28by%20ref%29) (InstigatedBy :type Controller%20Object%20Reference) (DamageCauser :type Actor%20Object%20Reference))
  (bind _normal (Collision|BreakHitResult HitInfo))
  (bind _returnvalue (Math|Vector|NegateVector _normal))
  (bind _returnvalue_2 (* _returnvalue 1e+03))
  (bind (_x _y _z) (Math|Vector|BreakVector _returnvalue_2))
  (bind _returnvalue_3 (Math|Float|Clamp(Float) _z 1e+02 2e+03))
  (bind _returnvalue_4 (Math|Vector|MakeVector _x _y _returnvalue_3))
  (CallFunction|TurnOffFriction)
  (Development|PrintString (Utilities|String|ToString(Vector) _returnvalue_4))
  (Physics|AddImpulse (Variables|Character|GetCharacterMovement) _returnvalue_4 true)
  (Utilities|Time|SetTimerbyEvent (EventDispatchers|CreateEvent :!event ResumeFriction) 1.0))

(fn TurnOffFriction
  (bind _charactermovement (Variables|Character|GetCharacterMovement))
  (Variables|/Script/Engine.CharacterMovementComponent|SetBrakingFrictionFactor _charactermovement 0.0)
  (Variables|/Script/Engine.CharacterMovementComponent|SetBrakingDecelerationWalking _charactermovement (Variables|/Script/Engine.CharacterMovementComponent|GetBrakingDecelerationFalling _charactermovement)))

(fn ResumeFriction
  (bind _charactermovement (Variables|Character|GetCharacterMovement))
  (Variables|/Script/Engine.CharacterMovementComponent|SetBrakingFrictionFactor _charactermovement (Variables|Default|GetOrigFrictionFactor))
  (Variables|/Script/Engine.CharacterMovementComponent|SetBrakingDecelerationWalking _charactermovement (Variables|Default|GetOrigDeceleraion)))