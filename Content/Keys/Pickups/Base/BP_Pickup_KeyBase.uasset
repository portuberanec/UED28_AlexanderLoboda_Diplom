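; Base Blueprint for key pickups that grant a key to the actor collecting them.
; It implements ActivatePickupEffect, which checks that its Key class is valid, adds it to the BPAC_KeyRing component found on that actor, then destroys the pickup.
; The key ring lookup has no validity check, and the event graph and construction script add no logic of their own.
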(event EventBeginPlay
  (|CallParentFunction) ; This node is disabled and will not be called.\nDrag off pins to build functionality.
)

(event Collision|EventActorBeginOverlap
  (params (OtherActor :type Actor%20Object%20Reference))
  (|CallParentFunction OtherActor) ; This node is disabled and will not be called.\nDrag off pins to build functionality.
)

(event EventTick
  (params (DeltaSeconds :type Float%20%28single-precision%29))
  (|CallParentFunction DeltaSeconds) ; This node is disabled and will not be called.\nDrag off pins to build functionality.
)

(fn ConstructionScript
  (|CallParentFunction))

(fn ActivatePickupEffect
  (params (InActor :type Actor%20Object%20Reference))
  (if (Utilities|IsValidClass (Variables|Default|GetKey))
    (Default|AddKey (Actor|GetComponentbyClass InActor "/Game/Character/Components/BPAC_KeyRing.BPAC_KeyRing_C") (Variables|Default|GetKey))
    (Actor|DestroyActor)))