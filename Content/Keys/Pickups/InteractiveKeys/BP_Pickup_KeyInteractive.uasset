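; Interactive key pickup that activates when it receives an interact message, passing the interactor along to ActivatePickup.
; Overlapping its collision sphere adds the pickup to the other actor's BPAC_Interaction_Simple queue, if that component exists, and ending overlap removes it.
; The construction script defers to the parent.
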(event OnComponentBeginOverlap(SphereCollision)
  (params (OverlappedComponent :type Primitive%20Component%20Object%20Reference) (OtherActor :type Actor%20Object%20Reference) (OtherComp :type Primitive%20Component%20Object%20Reference) (OtherBodyIndex :type Integer) (bFromSweep :type Boolean) (SweepResult :type Hit%20Result%20Structure%20%28by%20ref%29))
  (bind _returnvalue (Actor|GetComponentbyClass OtherActor "/Game/ComponentsCommon/BPAC_Interaction_Simple.BPAC_Interaction_Simple_C"))
  (Utilities|IsValid _returnvalue
    (:Is%20Valid
      (Default|AddtoQueue _returnvalue self))))

(event OnComponentEndOverlap(SphereCollision)
  (params (OverlappedComponent :type Primitive%20Component%20Object%20Reference) (OtherActor :type Actor%20Object%20Reference) (OtherComp :type Primitive%20Component%20Object%20Reference) (OtherBodyIndex :type Integer))
  (bind _returnvalue (Actor|GetComponentbyClass OtherActor "/Game/ComponentsCommon/BPAC_Interaction_Simple.BPAC_Interaction_Simple_C"))
  (Utilities|IsValid _returnvalue
    (:Is%20Valid
      (Default|RemovefromQueue _returnvalue self))))

(event EventInteractMessage
  (params (Interactor :type Actor%20Object%20Reference))
  (CallFunction|ActivatePickup Interactor))

(fn ConstructionScript
  (|CallParentFunction))